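; Player-controllable tank Blueprint that binds input to aiming, firing and tracked movement.
; BeginPlay hands the barrel and turret to the aiming component, and both tracks to the movement component.
; Axis input rotates the azimuth gimbal and spring arm, and drives tracks either by direct per-track throttle or movement-component intents.
; The construction script sets meshes, socket-attaches barrel to turret, and assigns the aiming component only if attachment succeeds.
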(event `self.ReceiveBeginPlay`
  (bind _output_get (set `self.m_Barrel` (`self.TankBarrel`)))
  (`TankAimingComponent.Initialize` (`self.TankAimingComponent`) _output_get (`self.TankTurret1`))
  (`TankMovementComponent.Initialize` (`self.TankMovement`) (`self.TankTrackL`) (`self.TankTrackR`)))

(event `InputAxis|Azimuth`
  (params (AxisValue :type "Float (single-precision)"))
  ;[1 1 1] MouseAiming
  (`SceneComponent.K2_AddLocalRotation` (`self.AzimuthGimbal`) (`KismetMathLibrary.MakeRotator` 0.0 0.0 (* AxisValue (`GameplayStatics.GetWorldDeltaSeconds`) 100.0)) false false))

(event `InputAxis|Altitude`
  (params (AxisValue :type "Float (single-precision)"))
  ;[1 1 1] MouseAiming
  (`SceneComponent.K2_AddLocalRotation` (`self.SpringArm`) (`KismetMathLibrary.MakeRotator` 0.0 (* AxisValue (`GameplayStatics.GetWorldDeltaSeconds`) 100.0)) false false))

(event `InputAction|Fire`
  (params (Key :type "Key Structure"))
  ;[1 1 1] Firing
  (:`Pressed`
    (`self.Fire`)))

(event `InputAxis|Left Track Throttle`
  (params (AxisValue :type "Float (single-precision)"))
  ;[1 1 1] Movement
  (`TankTrack.setThrottle` (`self.TankTrackL`) AxisValue))

(event `InputAxis|Right Track Throttle`
  (params (AxisValue :type "Float (single-precision)"))
  ;[1 1 1] Movement
  (`TankTrack.setThrottle` (`self.TankTrackR`) AxisValue))

(event `InputAxis|ForwardBackwardIntent`
  (params (AxisValue :type "Float (single-precision)"))
  ;[1 1 1] Movement
  (`TankMovementComponent.IntendMoveForward` (`self.TankMovement`) AxisValue))

(event `InputAxis|RightLeftTurnIntend`
  (params (AxisValue :type "Float (single-precision)"))
  ;[1 1 1] Movement
  (`TankMovementComponent.IntendTurnRight` (`self.TankMovement`) AxisValue))

(fn `UserConstructionScript`
  (`StaticMeshComponent.SetStaticMesh` (`self.TankTrackL`) null)
  (`StaticMeshComponent.SetStaticMesh` (`self.TankTrackR`) null)
  (`StaticMeshComponent.SetStaticMesh` (`self.TankBarrel`) "/Game/Tank/tank_fbx_Barrel.tank_fbx_Barrel")
  (`StaticMeshComponent.SetStaticMesh` (`self.TankTurret1`) "/Game/Tank/tank_fbx_Turret.tank_fbx_Turret")
  (bind _returnvalue (`SceneComponent.K2_AttachToComponent` (`self.TankBarrel`) (`self.TankTurret1`) "Barrel" "KeepRelative" "KeepRelative" "KeepRelative" true))
  (if _returnvalue
    (set `self.TankAimingComponent` (`self.TankAiming`))
    (else
      (`KismetSystemLibrary.PrintText` "Hello"))))