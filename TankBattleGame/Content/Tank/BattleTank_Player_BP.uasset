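; BattleTank_Player_BP is the player's tank Blueprint, configuring the tank's loadout and durability at startup.
; On BeginPlay it calls the parent event, assigns the heavy projectile to the TankAiming component, then sets starting health and the aiming component's reload time.
; It adds no other logic: the construction script only calls its parent, and the overlap and tick events are disabled.
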(event `self.ReceiveBeginPlay`
  (`parent.ReceiveBeginPlay`)
  (`TankAimingComponent.setProjectile` (`self.TankAiming`) "/Game/Projectile/Heavy_Projectile_BP.Heavy_Projectile_BP_C")
  (set `self.m_StartingHealth` 150)
  (set `TankAimingComponent.m_ReloadTimeInSeconds` 2.0 (`self.TankAiming`)))

(fn `UserConstructionScript`
  (`parent.UserConstructionScript`))