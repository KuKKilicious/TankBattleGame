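; Large tank Blueprint variant that ends the match as won for the player when its health runs out.
; BeginPlay runs the parent setup, then configures aiming with the heavy projectile and its own reload, ammo and velocity, along with starting health and minimum barrel elevation.
; Tick polls health percent and, at zero or below, calls GameOver on the BattleTankGame mode with the won reason.
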(event `self.ReceiveBeginPlay`
  (bind _tankaiming (`self.TankAiming`))
  (`parent.ReceiveBeginPlay`)
  (`TankAimingComponent.setProjectile` (`self.TankAiming`) "/Game/Projectile/Heavy_Projectile_BP.Heavy_Projectile_BP_C")
  (set `TankAimingComponent.m_ReloadTimeInSeconds` 3.0 _tankaiming)
  (set `TankAimingComponent.m_AmmoCount` 50 _tankaiming)
  (set `TankAimingComponent.m_FiringVelocity` 9000.0 _tankaiming)
  (set `self.m_StartingHealth` 200)
  (set `TankBarrel.m_MinimumElevation` -25.0 (`self.TankBarrel`)))

(event `self.ReceiveTick`
  (params (DeltaSeconds :type "Float (single-precision)"))
  (if (<= (`self.getHealthPercent`) 0.0)
    (bind _asbattle_tank_game (cast `/Game/Blueprints/BattleTankGame` (`GameplayStatics.GetGameMode`)))
    (`/Game/Blueprints/BattleTankGame.GameOver` _asbattle_tank_game null "GameOverWon")))

(fn `UserConstructionScript`
  (`parent.UserConstructionScript`))