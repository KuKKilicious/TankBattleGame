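; BattleTankGame runs the tank match flow: it shows timed instructions at start, counts down a clock and ends the game on timeout or death.
; Tick uses a one-second Delay to step the minutes/seconds countdown, then checks for expiry (BattlegroundLowPoly level only) or zero tank health.
; GameOver shows a reason-specific UI, disables tank movement and switches to mouse-driven UI input.
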(event `self.ReceiveBeginPlay`
  (set `self.Minutes` (`self.StartMinutes`))
  (bind _returnvalue (`|CreateWidget` "/Game/UI/InstructionsUI.InstructionsUI_C" (`GameplayStatics.GetPlayerController` 0)))
  (`UserWidget.AddToViewport` _returnvalue 0)
  (`KismetSystemLibrary.Delay` 7.0)
  (`Widget.SetVisibility` _returnvalue "Hidden"))

(event `self.ReceiveTick`
  (params (DeltaSeconds :type "Float (single-precision)"))
  (bind _returnvalue (and (== (`self.Seconds`) 0) (== (`self.Minutes`) 0)))
  (if (and (not (`self.isGameOver`)) (not _returnvalue))
    (`KismetSystemLibrary.Delay` 1.0)
    (`self.CountDownSecondsMinutes`)
    (if _returnvalue
      (bind _returnvalue_2 (`GameplayStatics.GetCurrentLevelName` true))
      (bind _astank_game_instance (cast `/Game/UI/TankGameInstance` (`GameplayStatics.GetGameInstance`))
        (:`then`
          (if (`KismetStringLibrary.EqualEqual_StrStr` _returnvalue_2 "BattlegroundLowPoly")
            (`/Engine/EditorBlueprintResources/StandardMacros.DoOnce` false
              (:`Completed`
                (`self.GameOver` _astank_game_instance "GameOverTime")))))
        (:`CastFailed`
          (`KismetSystemLibrary.PrintString` "Cast failed: No TankGameInstance")))
      (else
        (bind _astank (cast `Tank` (`GameplayStatics.GetPlayerPawn` 0)))
        (if (<= (`Tank.getHealthPercent` _astank) 0.0)
          (`/Engine/EditorBlueprintResources/StandardMacros.DoOnce` false
            (:`Completed`
              (`self.GameOver` null "GameOverDied"))))))))

(fn `CountDownSecondsMinutes`
  (if (== (`self.Seconds`) 0)
    (set `self.Seconds` 59)
    (`/Engine/EditorBlueprintResources/StandardMacros.DecrementInt` (`self.Minutes`))
    (else
      (`/Engine/EditorBlueprintResources/StandardMacros.DecrementInt` (`self.Seconds`)))))

(fn `CountUpSecondsMinutes`
  (if (== (`self.Seconds`) 59)
    (set `self.Seconds` 0)
    (`/Engine/EditorBlueprintResources/StandardMacros.IncrementInt` (`self.Minutes`))
    (else
      (`/Engine/EditorBlueprintResources/StandardMacros.IncrementInt` (`self.Seconds`)))))

(fn `GameOver`
  (params (self2 :type "/Game/UI/TankGameInstance Object Reference") (GameOverReason :type String))
  (bind _returnvalue (`GameplayStatics.GetPlayerController` 0))
  (set `self.isGameOver` true)
  (bind _returnvalue_2 (`|CreateWidget` "/Game/UI/GameOverUI.GameOverUI_C"))
  (set `/Game/UI/GameOverUI.GameOverReason` GameOverReason _returnvalue_2)
  (`UserWidget.AddToViewport` _returnvalue_2 0)
  (`TankMovementComponent.disableMovement` (`self.GetComponentByClass` (`GameplayStatics.GetPlayerPawn` 0) "/Script/TankBattleGame.TankMovementComponent"))
  (`WidgetBlueprintLibrary.SetInputMode_UIOnlyEx` _returnvalue null)
  (set `PlayerController.bShowMouseCursor` true _returnvalue))

(fn `Set Score`
  (params (self2 :type "/Game/UI/TankGameInstance Object Reference")))

(fn `UserConstructionScript`
  (`self.Set Score` null))